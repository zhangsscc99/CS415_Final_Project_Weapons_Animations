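; Melee enemy spawner that periodically creates pairs of BP_EnemyMelee at its Sphere component and sends them after the player.
; Tick increments TimeToSpawn by one per frame and resets it at a fixed count, so the spawn interval depends on frame rate.
; Each spawn sets AI_Enemy as the controller class after spawning, then calls AIMoveTo targeting the player character.
; The second spawn chains directly from the first move call's immediate output.
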(event EventTick
  (params (DeltaSeconds :type Float%20%28single-precision%29))
  (bind _sphere (Variables|Default|GetSphere))
  (bind _sphere_2 (Variables|Default|GetSphere))
  (if (== 5.4e+02 (Variables|Default|GetTimeToSpawn))
    (Variables|Default|SetTimeToSpawn 0.0)
    (bind _returnvalue (Game|SpawnActorfromClass "/Game/TopDown/Blueprints/Characters/BP_EnemyMelee.BP_EnemyMelee_C" (Math|Transform|MakeTransform (Transformation|GetWorldLocation _sphere) (Transformation|GetWorldRotation _sphere) "1.000000,1.000000,1.000000") "Undefined" 0 0))
    (Variables|/Script/Engine.Pawn|SetAIControllerClass _returnvalue "/Game/Blueprints/AI_Enemy.AI_Enemy_C")
    (AI|AIMoveTo _returnvalue "0, 0, 0" (Game|GetPlayerCharacter 0) 5.0 false
      (:then
        (bind _returnvalue_2 (Game|SpawnActorfromClass "/Game/TopDown/Blueprints/Characters/BP_EnemyMelee.BP_EnemyMelee_C" (Math|Transform|MakeTransform (Transformation|GetWorldLocation _sphere_2) (Transformation|GetWorldRotation _sphere_2) "1.000000,1.000000,1.000000") "Undefined" 0 0))
        (Variables|/Script/Engine.Pawn|SetAIControllerClass _returnvalue_2 "/Game/Blueprints/AI_Enemy.AI_Enemy_C")
        (AI|AIMoveTo _returnvalue_2 "0, 0, 0" (Game|GetPlayerCharacter 0) 5.0 false)))
    (else
      (Variables|Default|SetTimeToSpawn (+ (Variables|Default|GetTimeToSpawn) 1.0)))))

(fn ConstructionScript)